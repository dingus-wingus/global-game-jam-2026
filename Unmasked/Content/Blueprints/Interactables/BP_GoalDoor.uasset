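; BP_GoalDoor is an interactable exit door that loads the level named by LevelName when the player passes a retinal scan.
; The scan passes only if the player's PaperZD anim instance class is ABP_AltGaurd, so the active animation blueprint acts as the credential; otherwise it prints a failure.
; Separate OpenDoor and CloseDoor events set IsOpen and swing the door's yaw with a reversible timeline, independently of Interact.
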(event `OpenDoor`
  (set `self.IsOpen` true)
  (bind (_direction _zrotation) (`Timeline|OpenDoor Timeline` :!label _label)
    (:`Update`
      (`SceneComponent.K2_SetRelativeRotation` (`self.Door`) (`KismetMathLibrary.MakeRotator` 0.0 0.0 _zrotation) false false))))

(event `CloseDoor`
  (set `self.IsOpen` false)
  (goto _label :!via `Reverse`))

(event `self.Interact`
  (params (Interactor :type "Actor Object Reference"))
  (bind _asbp_player (cast `/Game/Blueprints/Player/BP_Player` Interactor))
  (if (== (`GameplayStatics.GetObjectClass` (`PaperZDAnimationComponent.AnimInstance` (`self.GetComponentByClass` _asbp_player "/Script/PaperZD.PaperZDAnimationComponent"))) "/Game/AI/ABP_AltGaurd.ABP_AltGaurd_C")
    (`GameplayStatics.OpenLevel` (`self.Level Name`))
    (else
      (`KismetSystemLibrary.PrintString` "Retinal Scan Failed!" true true (struct :`R` 1.0 :`A` 1.0)))))

(fn `UserConstructionScript`)