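; BP_Player is the player character, with isometric-style movement, a pause menu and a timed disguise.
; Enhanced Input drives movement rotated 45 degrees from control yaw and the pause toggle, while the dash action only emits noise.
; SetDisguise swaps the PaperZD animation instance class and shows a widget bar, which Tick counts down before restoring the default animation.
; Die prints a message and reloads the current level.
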(event `self.ReceiveBeginPlay`
  (`EnhancedInputSubsystemInterface.AddMappingContext` (pcsubsystem `EnhancedInputLocalPlayerSubsystem` (`GameplayStatics.GetPlayerController` 0)) "/Game/Variant_TwinStick/Input/IMC_TwinStick.IMC_TwinStick" 0 (struct))
  (bind _aswbp_disguise (cast `/Game/Blueprints/Player/WBP_Disguise` (`WidgetComponent.GetWidget` (`self.DisguiseWidget`))))
  (bind _output_get (set `self.Disguise Bar` (`/Game/Blueprints/Player/WBP_Disguise.DisguiseBar` _aswbp_disguise)))
  (`Widget.SetVisibility` _output_get "Hidden"))

(event `EnhancedInput|/Game/Variant_TwinStick/Input/Actions/IA_Action_Move`
  (params (ActionValue :type "Vector2D Structure") (ElapsedSeconds :type "Float (double-precision)") (TriggeredSeconds :type "Float (double-precision)") (InputAction :type "InputAction Object Reference" :default "/Game/Variant_TwinStick/Input/Actions/IA_Action_Move.IA_Action_Move"))
  (:`Triggered`
    (`self.Move` ActionValue_X ActionValue_Y)))

(event `EnhancedInput|/Game/Variant_TwinStick/Input/Actions/IA_Action_Dash`
  (params (ActionValue :type Boolean) (ElapsedSeconds :type "Float (double-precision)") (TriggeredSeconds :type "Float (double-precision)") (InputAction :type "InputAction Object Reference" :default "/Game/Variant_TwinStick/Input/Actions/IA_Action_Dash.IA_Action_Dash"))
  (:`Triggered`
    (`self.MakeNoise` 1.0 null (`self.K2_GetActorLocation`))))

(event `EnhancedInput|/Game/Variant_TwinStick/Input/Actions/IA_PauseGame`
  (params (ActionValue :type Boolean) (ElapsedSeconds :type "Float (double-precision)") (TriggeredSeconds :type "Float (double-precision)") (InputAction :type "InputAction Object Reference" :default "/Game/Variant_TwinStick/Input/Actions/IA_PauseGame.IA_PauseGame"))
  (bind _returnvalue (`GameplayStatics.GetPlayerController` 0))
  (bind _pausewidget (`self.PauseWidget`))
  (:`Started`
    (if (not (`self.Paused?`))
      (set `self.Paused?` true)
      (bind _returnvalue_2 (`|CreateWidget` "/Game/UI/WB_PauseMenu.WB_PauseMenu_C" _returnvalue))
      (bind _output_get (set `self.PauseWidget` _returnvalue_2))
      (`UserWidget.AddToViewport` _output_get 0)
      (`WidgetBlueprintLibrary.SetInputMode_GameAndUIEx` _returnvalue _pausewidget)
      (set `PlayerController.bShowMouseCursor` true (`GameplayStatics.GetPlayerController` 0))
      (`GameplayStatics.SetGamePaused` true)
      (else
        (set `self.Paused?` false)
        (`Widget.RemoveFromParent` _pausewidget)
        (`WidgetBlueprintLibrary.SetInputMode_GameOnly` _returnvalue)
        (set `PlayerController.bShowMouseCursor` false _returnvalue)
        (`GameplayStatics.SetGamePaused` false)))))

(event `self.ReceiveTick`
  (params (DeltaSeconds :type "Float (single-precision)"))
  (if (`self.Disguised`)
    (if (<= (`self.CurrentDisguiseTimer`) 0.0)
      (set `self.Disguised` false)
      (`PaperZDAnimationComponent.SetAnimInstanceClass` (`self.Animation`) "/Game/Blueprints/Player/ABP_Player.ABP_Player_C")
      (`Widget.SetVisibility` (`self.Disguise Bar`) "Hidden")
      (else
        (set `self.CurrentDisguiseTimer` (- (`self.CurrentDisguiseTimer`) (`GameplayStatics.GetWorldDeltaSeconds`)))
        (`ProgressBar.SetPercent` (`self.Disguise Bar`) (/ (`self.CurrentDisguiseTimer`) (`self.MaxDisguiseTimer`)))))))

(fn `Die`
  (`KismetSystemLibrary.PrintString` "You Died!")
  (bind _returnvalue (`GameplayStatics.GetCurrentLevelName` true))
  (`GameplayStatics.OpenLevel` (`KismetStringLibrary.Conv_StringToName` _returnvalue)))

(fn `Move`
  (params (X :type "Float (double-precision)") (Y :type "Float (double-precision)"))
  (bind (_returnvalue_roll _returnvalue_pitch _returnvalue_yaw) (`KismetMathLibrary.BreakRotator` (`self.GetControlRotation`)))
  (bind (_returnvalue_roll_2 _returnvalue_pitch_2 _returnvalue_yaw_2) (`KismetMathLibrary.BreakRotator` (`self.GetControlRotation`)))
  (`self.AddMovementInput` (`KismetMathLibrary.GetForwardVector` (`KismetMathLibrary.MakeRotator` _returnvalue_roll_2 0.0 (+ _returnvalue_yaw_2 45.0))) X)
  (`self.AddMovementInput` (`KismetMathLibrary.GetRightVector` (`KismetMathLibrary.MakeRotator` _returnvalue_roll 0.0 (+ _returnvalue_yaw 45.0))) Y))

(fn `SetDisguise`
  (params (`Anim BP` :type "PaperZDAnimInstance Class Reference"))
  (`PaperZDAnimationComponent.SetAnimInstanceClass` (`self.Animation`) `Anim BP`)
  (set `self.Disguised` true)
  (set `self.CurrentDisguiseTimer` (`self.MaxDisguiseTimer`))
  (`Widget.SetVisibility` (`self.Disguise Bar`) "Visible"))

(fn `UserConstructionScript`)