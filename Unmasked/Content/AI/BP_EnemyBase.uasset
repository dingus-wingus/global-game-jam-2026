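; BP_EnemyBase is the base enemy character, providing the body-side actions and queries for an enemy AI.
; Attack plays a montage and signals attack end on completion or interruption, while Interact tells the AIC_EnemyBase controller to enter its dead state.
; Tick decays the detection level over time.
; Helper functions check the sphere for an overlapping player, expose the patrol route, and switch walk speed between roaming and chasing.
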(event `Attack`
  (`|PlayMontage` (`self.Mesh`) "/Game/AI/Animations/MNTG_Attack.MNTG_Attack"
    (:`OnCompleted`
      _)
    (:`OnInterrupted`
      _))
  (`self.OnAttackEnd`))

(event `/Game/Blueprints/Player/BPI_Interactable.Interact`
  (params (Interactor :type "Actor Object Reference"))
  (`KismetSystemLibrary.PrintString` "Enemy Hit!")
  (bind _asaic_enemy_base (cast `/Game/AI/AIC_EnemyBase` (`AIBlueprintHelperLibrary.GetAIController` self)))
  (`/Game/AI/AIC_EnemyBase.SetStateDead` _asaic_enemy_base))

(event `self.ReceiveTick`
  (params (DeltaSeconds :type "Float (single-precision)"))
  (if (> (`self.CurrentDetection`) 0.0)
    (set `self.CurrentDetection` (- (`self.CurrentDetection`) (* (`self.DetectionDecayRate`) (`GameplayStatics.GetWorldDeltaSeconds`))))))

(fn `CheckForOverlappingPlayer`
  (returns (Player :type "/Game/Blueprints/Player/BP_Player Object Reference") (Succeeded :type Boolean))
  (for _array_element (`PrimitiveComponent.GetOverlappingActors` (`self.Sphere`) "/Game/Blueprints/Player/BP_Player.BP_Player_C")
    (bind _asbp_player (cast `/Game/Blueprints/Player/BP_Player` _array_element)
      (:`then`
        (return _asbp_player true))
      (:`CastFailed`
        (return null false)))))

(fn `GetPatrolRoute`
  (returns (PatrolRoute :type "/Game/AI/BP_PatrolRoute Object Reference"))
  (return (`self.PatrolRoute`)))

(fn `SetMovementSpeed`
  (params (Speed :type "/Game/AI/Enums/E_MovementSpeed Enum" :default "NewEnumerator0"))
  (returns (SpeedValue :type "Float (double-precision)"))
  (bind _output_get (set `CharacterMovementComponent.MaxWalkSpeed` (select `/Game/AI/Enums/E_MovementSpeed` Speed :`NewEnumerator0` 200.0 :`NewEnumerator1` 600.0 :!type "Float (single-precision)") (`self.CharacterMovement`)))
  (return _output_get))

(fn `UserConstructionScript`)