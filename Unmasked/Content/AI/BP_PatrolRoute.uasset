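; BP_PatrolRoute is an AI patrol route actor that defines waypoints as the points of a PatrolRoute spline.
; GetSplinePointAsWorldPosition returns the world location of the point at the current PatrolIndex.
; IncrementPatrolRoute adds Direction to that index and resets it to zero at the point count, looping the route.
; Only the upper end wraps; negative indices are not handled.
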(event `IncrementPatrolRoute`
  (bind _output_get (set `self.PatrolIndex` (+ (`self.PatrolIndex`) (`self.Direction`))))
  (if (== _output_get (`SplineComponent.GetNumberOfSplinePoints` (`self.PatrolRoute`)))
    (set `self.PatrolIndex` 0)))

(fn `GetSplinePointAsWorldPosition`
  (returns (Location :type "Vector Structure"))
  (return (`SplineComponent.GetLocationAtSplinePoint` (`self.PatrolRoute`) (`self.PatrolIndex`) "World")))

(fn `UserConstructionScript`)